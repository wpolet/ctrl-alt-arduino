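; Player Blueprint for a timed Simon-style memory game with five colored point lights, played through an Arduino over serial.
; Each turn appends a random light and blinks the sequence back with a recursive delayed event.
; Input from serial lines polled on Tick, or test letter keys, is compared recursively once lengths match.
; A match updates the goal text and advances until the target; a mistake or expired countdown ends the game.
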(event Custom|StartGame
  ;[1 1 1] Start the game
  (for _array_element (Variables|Default|GetArrayPointLights)
    (Rendering|SetVisibility _array_element true false))
  (Utilities|FlowControl|Delay 1.0)
  (for _array_element_2 (Variables|Default|GetArrayPointLights)
    (Rendering|SetVisibility _array_element_2 false false))
  (Utilities|FlowControl|Delay 1.0)
  (Development|PrintString "Loops completed")
  (Utilities|FlowControl|DoOnce false
    (:Completed
      (bind _returnvalue (Utilities|Time|SetTimerbyEvent (delegate Custom|SetTimer) 1.0 true))
      (Variables|Default|SetIsGameStarted true)
      (Utilities|Array|Clear (Variables|Default|GetRandomIntSequence))
      (CallFunction|NewTurn))))

(event Custom|SetTimer
  ;[1 1 1] Start the game
  (if (> (Variables|Default|GetSecondsLeft) 0)
    (Variables|Default|SetSecondsLeft (- (Variables|Default|GetSecondsLeft) 1))
    (if (Variables|Default|GetIsGameStarted)
      (if (< (Variables|Default|GetSecondsLeft) 10)
        (Variables|Default|SetStringTimeLeft (Utilities|String|Append (Utilities|String|ToString(Integer) (/ (Variables|Default|GetSecondsLeft) 60)) ":" (Utilities|String|Append "0" (Utilities|String|ToString(Integer) (Math|Integer|%(Integer) (Variables|Default|GetSecondsLeft) 60)))))
        (else
          (Variables|Default|SetStringTimeLeft (Utilities|String|Append (Utilities|String|ToString(Integer) (/ (Variables|Default|GetSecondsLeft) 60)) ":" (Utilities|String|ToString(Integer) (Math|Integer|%(Integer) (Variables|Default|GetSecondsLeft) 60))))))
      (Rendering|Components|TextRender|SetText (Variables|Default|GetChrono) (Utilities|Text|ToText(String) (Variables|Default|GetStringTimeLeft))))
    (else
      (Utilities|Time|ClearandInvalidateTimerbyHandle (stale Custom|StartGame _returnvalue))
      (CallFunction|GameOver))))

(event Custom|NewTurn
  ;[1 1 1] New turn: select a random light to add to the sequence
  (Utilities|Array|Clear (Variables|Default|GetPlayerColorSequence))
  (Utilities|Array|Add (Variables|Default|GetRandomIntSequence) (Math|Random|RandomInteger 5))
  (CallFunction|BlinktheLights))

(event Custom|BlinkTheLights
  (params (Index :type Integer))
  (bind _randomintsequence (Variables|Default|GetRandomIntSequence))
  (bind _arraypointlights (Variables|Default|GetArrayPointLights))
  (bind _output (Utilities|Array|Get(acopy) _randomintsequence Index))
  (bind _output_2 (Utilities|Array|Get(acopy) _arraypointlights _output))
  ;[1 1 1] Blink the lights of the sequence in order
  (if (< Index (Utilities|Array|Length _randomintsequence))
    (Rendering|SetVisibility _output_2 true false)
    (Utilities|FlowControl|Delay 0.5)
    (Rendering|SetVisibility _output_2 false false)
    (Utilities|FlowControl|Delay 0.5)
    (bind _result (Math|Integer|IncrementInt Index)
      (:%20%20
        (CallFunction|BlinktheLights _result)))))

(event Custom|GameOver
  ;[1 1 1] Game Over
  (Variables|Default|SetIsGameStarted false)
  (for _array_element (Variables|Default|GetArrayPointLights)
    (Rendering|SetVisibility _array_element false false))
  (Development|PrintString "Game Over"))

(event Custom|CheckSequence
  ;[1 1 1] Compare Color sequence with sequence given by the player
  (Variables|Default|SetIsSequenceCorrect true)
  (CallFunction|CheckSequenceItem)
  (if (Variables|Default|GetIsSequenceCorrect)
    (Audio|PlaySound2D "/Game/Sounds/S_Correct.S_Correct" 1.0 1.0 0.0 0 0)
    (bind _result (Math|Integer|IncrementInt (Variables|Default|GetCurrentLightIndex))
      (:%20%20
        (Rendering|Components|TextRender|SetText (Variables|Default|GetGoal) (Utilities|Text|ToText(String) (Utilities|String|Append (Utilities|String|ToString(Integer) _result) "/" (Utilities|String|ToString(Integer) (Variables|Default|GetMaxLightIndex)))))
        (Utilities|FlowControl|Delay 1.0)
        (if (== (Variables|Default|GetCurrentLightIndex) (Variables|Default|GetMaxLightIndex))
          (Development|PrintString "You Win!")
          (else
            (CallFunction|NewTurn)))))
    (else
      (Audio|PlaySound2D "/Game/Sounds/S_Error.S_Error" 1.0 1.0 0.0 0 0)
      (Development|PrintString "Incorrect sequence")
      (CallFunction|GameOver))))

(event Custom|CheckSequenceItem
  (params (Index :type Integer))
  (bind _randomintsequence (Variables|Default|GetRandomIntSequence))
  ;[1 1 1] Compare each element of both sequences
  (if (< Index (Utilities|Array|Length _randomintsequence))
    (if (Utilities|Enum|Equal(Enum) (Utilities|Array|Get(acopy) (Variables|Default|GetPlayerColorSequence) Index) (Utilities|Array|Get(acopy) (Variables|Default|GetArrayStrings) (Utilities|Array|Get(acopy) _randomintsequence Index)))
      (bind _result (Math|Integer|IncrementInt Index)
        (:%20%20
          (CallFunction|CheckSequenceItem _result)))
      (else
        (Variables|Default|SetIsSequenceCorrect false)))))

(event EventTick
  (params (DeltaSeconds :type Float%20%28single-precision%29))
  (bind _playercolorsequence (Variables|Default|GetPlayerColorSequence))
  (bind _arduino (Variables|Default|GetArduino))
  (if (Variables|Default|GetIsGameStarted)
    ;[1 1 1] Recieve Command from Arduino Serial
    (Utilities|IsValid _arduino
      (:Is%20Valid
        (bind (_bsuccess _returnvalue) (Class|Serial|Readln _arduino))
        (Development|PrintString _returnvalue)
        (if _bsuccess
          (Utilities|Array|Add _playercolorsequence _returnvalue)
          (if (== (Utilities|Array|Length _playercolorsequence) (Utilities|Array|Length (Variables|Default|GetRandomIntSequence)))
            (CallFunction|CheckSequence))))
      (:Is%20Not%20Valid
        (Development|PrintString "Arduino Object Not valid")))))

(event EventEndPlay
  (params (EndPlayReason :type EEndPlayReason%20Enum :default "Destroyed"))
  (bind _arduino (Variables|Default|GetArduino))
  ;[1 1 1] Close Serial Port
  (Utilities|IsValid _arduino
    (:Is%20Valid
      (Class|Serial|Close _arduino))))

(event EventBeginPlay
  ;[1 1 1] Event begin play: turn off all lights and associates a color to each light
  (Input|EnableInput (Game|GetPlayerController 0))
  (bind _output_get (Variables|Default|SetArrayPointLights (Utilities|Array|MakeArray (Variables|Default|GetPointLight1) (Variables|Default|GetPointLight2) (Variables|Default|GetPointLight3) (Variables|Default|GetPointLight4) (Variables|Default|GetPointLight5))))
  (for (_array_element _array_index) _output_get
    (Rendering|Components|Light|SetLightColor _array_element (Utilities|Array|Get(acopy) (Variables|Default|GetArrayColors) _array_index) false)
    (Rendering|SetVisibility _array_element false false))
  ;[1 1 1] Set Goal text render
  (bind _output_get_2 (Variables|Default|SetCurrentLightIndex 0))
  (Rendering|Components|TextRender|SetText (Variables|Default|GetGoal) (Utilities|Text|ToText(String) (Utilities|String|Append (Utilities|String|ToString(Integer) _output_get_2) "/" (Utilities|String|ToString(Integer) (Variables|Default|GetMaxLightIndex)))))
  ;[1 1 1] Open Serial Port to communicate with Arduino
  (bind (_bopened _returnvalue) (Class|Serial|OpenComPort 3 9600))
  (if _bopened
    (bind _output_get_3 (Variables|Default|SetArduino _returnvalue))
    (Class|Serial|Flush _output_get_3)
    (Development|PrintString "Port opened")
    (else
      (Development|PrintString "Port not opened"))))

(event Input|KeyboardEvents|Enter
  (params (Key :type Key%20Structure :default "None"))
  ;[1 0 0] Start the game for test
  (:Pressed
    (Development|PrintString "Enter pressed")
    ;[1 1 1] Start the game
    (for _array_element (Variables|Default|GetArrayPointLights)
      (Rendering|SetVisibility _array_element true false))
    (Utilities|FlowControl|Delay 1.0)
    (for _array_element_2 (Variables|Default|GetArrayPointLights)
      (Rendering|SetVisibility _array_element_2 false false))
    (Utilities|FlowControl|Delay 1.0)
    (Development|PrintString "Loops completed")
    (Utilities|FlowControl|DoOnce false
      (:Completed
        (bind _returnvalue (Utilities|Time|SetTimerbyEvent (delegate Custom|SetTimer) 1.0 true))
        (Variables|Default|SetIsGameStarted true)
        (Utilities|Array|Clear (Variables|Default|GetRandomIntSequence))
        (CallFunction|NewTurn)))))

(event Input|KeyboardEvents|W
  (params (Key :type Key%20Structure :default "None"))
  (bind _playercolorsequence (Variables|Default|GetPlayerColorSequence))
  ;[1 0 0] For Testing
  (:Pressed
    (Variables|Default|SetKeyStringToAdd "W")
    (if (Variables|Default|GetIsGameStarted)
      (Utilities|Array|Add _playercolorsequence (Variables|Default|GetKeyStringToAdd))
      (if (== (Utilities|Array|Length _playercolorsequence) (Utilities|Array|Length (Variables|Default|GetRandomIntSequence)))
        (CallFunction|CheckSequence)))))

(event Input|KeyboardEvents|G
  (params (Key :type Key%20Structure :default "None"))
  (bind _playercolorsequence (Variables|Default|GetPlayerColorSequence))
  ;[1 0 0] For Testing
  (:Pressed
    (Variables|Default|SetKeyStringToAdd "G")
    (if (Variables|Default|GetIsGameStarted)
      (Utilities|Array|Add _playercolorsequence (Variables|Default|GetKeyStringToAdd))
      (if (== (Utilities|Array|Length _playercolorsequence) (Utilities|Array|Length (Variables|Default|GetRandomIntSequence)))
        (CallFunction|CheckSequence)))))

(event Input|KeyboardEvents|B
  (params (Key :type Key%20Structure :default "None"))
  (bind _playercolorsequence (Variables|Default|GetPlayerColorSequence))
  ;[1 0 0] For Testing
  (:Pressed
    (Variables|Default|SetKeyStringToAdd "B")
    (if (Variables|Default|GetIsGameStarted)
      (Utilities|Array|Add _playercolorsequence (Variables|Default|GetKeyStringToAdd))
      (if (== (Utilities|Array|Length _playercolorsequence) (Utilities|Array|Length (Variables|Default|GetRandomIntSequence)))
        (CallFunction|CheckSequence)))))

(event Input|KeyboardEvents|R
  (params (Key :type Key%20Structure :default "None"))
  (bind _playercolorsequence (Variables|Default|GetPlayerColorSequence))
  ;[1 0 0] For Testing
  (:Pressed
    (Variables|Default|SetKeyStringToAdd "R")
    (if (Variables|Default|GetIsGameStarted)
      (Utilities|Array|Add _playercolorsequence (Variables|Default|GetKeyStringToAdd))
      (if (== (Utilities|Array|Length _playercolorsequence) (Utilities|Array|Length (Variables|Default|GetRandomIntSequence)))
        (CallFunction|CheckSequence)))))

(event Input|KeyboardEvents|Y
  (params (Key :type Key%20Structure :default "None"))
  (bind _playercolorsequence (Variables|Default|GetPlayerColorSequence))
  ;[1 0 0] For Testing
  (:Pressed
    (Variables|Default|SetKeyStringToAdd "Y")
    (if (Variables|Default|GetIsGameStarted)
      (Utilities|Array|Add _playercolorsequence (Variables|Default|GetKeyStringToAdd))
      (if (== (Utilities|Array|Length _playercolorsequence) (Utilities|Array|Length (Variables|Default|GetRandomIntSequence)))
        (CallFunction|CheckSequence)))))

(fn ConstructionScript)