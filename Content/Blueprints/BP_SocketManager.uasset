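; BP_SocketManager links the game to a Socket.IO server and forwards its events to the player Blueprint.
; On BeginPlay it binds the initEvent and moveEvent socket events to OnInit and OnMove, which call StartGame and GameOver on BPPlayer respectively.
; Connection, disconnection, failure and both game events print debug messages to the screen.
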(event OnConnected(SocketIOClient)
  (params (SessionId :type String) (bIsReconnection :type Boolean))
  (Development|PrintString "Connected"))

(event OnFail(SocketIOClient)
  (Development|PrintString "Fail"))

(event OnDisconnected(SocketIOClient)
  (params (Reason :type ESIOConnectionCloseReason%20Enum :default "CLOSE_REASON_NORMAL"))
  (Development|PrintString "Disconnected"))

(event Custom|OnMove
  (Development|PrintString "Perdu !")
  (Default|GameOver (Variables|Default|GetBP_Player)))

(event Custom|OnInit
  (Development|PrintString "Démarrage partie")
  (Default|StartGame (Variables|Default|GetBP_Player)))

(event EventBeginPlay
  (Development|PrintString "Trying to connect")
  (Class|SocketIOClientComponent|BindEventtoFunction (Variables|Default|GetSocketIOClient) "initEvent" "OnInit" 0 "/" "USE_DEFAULT") ; bind event to a bp function
  (Class|SocketIOClientComponent|BindEventtoFunction (Variables|Default|GetSocketIOClient) "moveEvent" "OnMove" 0 "/" "USE_DEFAULT"))

(fn ConstructionScript)